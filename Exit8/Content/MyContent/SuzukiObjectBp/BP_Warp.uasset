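; BP_Warp loops the player through an anomaly-check corridor, reporting each forward or turn-back choice to BP_FirstPersonGameMode via JugeChoice.
; Front overlap moves the player to the same relative offset at Back.
; Back overlap mirrors the offset around itself, flips yaw and control rotation, and restores negated XY velocity to keep movement seamless.
; Warps run only while ProgressCount is under 8; IsWarping blocks retriggers until WarpFlag overlap clears it.
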(event `self.Back.OnComponentBeginOverlap`
  (params (OverlappedComponent :type "PrimitiveComponent Object Reference") (OtherActor :type "Actor Object Reference") (OtherComp :type "PrimitiveComponent Object Reference") (OtherBodyIndex :type Integer) (bFromSweep :type Boolean) (SweepResult :type "HitResult Structure (by ref)"))
  (bind (_returnvalue_roll _returnvalue_pitch _returnvalue_yaw) (`KismetMathLibrary.BreakRotator` (`self.K2_GetActorRotation` OtherActor)))
  (bind _returnvalue (`GameplayStatics.GetPlayerController` 0))
  (bind (_returnvalue_roll_2 _returnvalue_pitch_2 _returnvalue_yaw_2) (`KismetMathLibrary.BreakRotator` (`Controller.GetControlRotation` _returnvalue)))
  ;[1 1 1] Backワープの当たり判定に触れた時、Playerの方向と位置を修正して、Backワープの位置に飛ばす
  (`GameplayStatics.GetAllActorsOfClass` "/Game/FirstPerson/Blueprints/BP_FirstPersonGameMode.BP_FirstPersonGameMode_C")
  (bind _asbp_first_person_game_mode (cast `/Game/FirstPerson/Blueprints/BP_FirstPersonGameMode` (`GameplayStatics.GetGameMode`))) ; GameModeより現在の正当数を取得
  (if (< (`/Game/FirstPerson/Blueprints/BP_FirstPersonGameMode.ProgressCount` _asbp_first_person_game_mode) 8)
    (if (not (`self.isWarping`))
      (set `self.isWarping` true) ; ワープ済みフラグを上げる
      (set `self.Velocity` (`MovementComponent.Velocity` (`Pawn.GetMovementComponent` (`GameplayStatics.GetPlayerPawn` 0))))
      (`self.K2_SetActorLocationAndRotation` OtherActor (+ (* (- (`self.K2_GetActorLocation` OtherActor) (`SceneComponent.K2_GetComponentLocation` (`self.Back`))) (-1.0 -1.0 1.0)) (`SceneComponent.K2_GetComponentLocation` (`self.Back`))) (`KismetMathLibrary.MakeRotator` _returnvalue_roll _returnvalue_pitch (+ _returnvalue_yaw 180.0)) false true)
      (`Controller.SetControlRotation` _returnvalue (`KismetMathLibrary.MakeRotator` _returnvalue_roll_2 _returnvalue_pitch_2 (+ _returnvalue_yaw_2 180.0)))
      (set `MovementComponent.Velocity` (* (`self.Velocity`) (-1.0 -1.0 1.0)) (`Pawn.GetMovementComponent` (`GameplayStatics.GetPlayerPawn` 0))) ; 反転すると速度が0になるので対策
      (bind _asbp_first_person_game_mode_2 (cast `/Game/FirstPerson/Blueprints/BP_FirstPersonGameMode` (`GameplayStatics.GetGameMode`)))
      (`/Game/FirstPerson/Blueprints/BP_FirstPersonGameMode.JugeChoice` _asbp_first_person_game_mode_2 false) ; ゲームモードに後退を選んだ回答を渡す
    )))

(event `self.Front.OnComponentBeginOverlap`
  (params (OverlappedComponent :type "PrimitiveComponent Object Reference") (OtherActor :type "Actor Object Reference") (OtherComp :type "PrimitiveComponent Object Reference") (OtherBodyIndex :type Integer) (bFromSweep :type Boolean) (SweepResult :type "HitResult Structure (by ref)"))
  ;[1 1 1] 前進のワープ当たり判定に触れた時、ゲームモードに前進した回答を渡し、Ｐｌａｙｅｒの開店と位置を修正して、Backワープの位置に戻す
  (`GameplayStatics.GetAllActorsOfClass` "/Game/FirstPerson/Blueprints/BP_FirstPersonGameMode.BP_FirstPersonGameMode_C")
  (bind _asbp_first_person_game_mode (cast `/Game/FirstPerson/Blueprints/BP_FirstPersonGameMode` (`GameplayStatics.GetGameMode`)))
  (if (< (`/Game/FirstPerson/Blueprints/BP_FirstPersonGameMode.ProgressCount` _asbp_first_person_game_mode) 8)
    (if (not (`self.isWarping`))
      (set `self.isWarping` true)
      (`self.K2_SetActorLocation` OtherActor (+ (- (`self.K2_GetActorLocation` OtherActor) (`SceneComponent.K2_GetComponentLocation` (`self.Front`))) (`SceneComponent.K2_GetComponentLocation` (`self.Back`))) false false)
      (bind _asbp_first_person_game_mode_2 (cast `/Game/FirstPerson/Blueprints/BP_FirstPersonGameMode` (`GameplayStatics.GetGameMode`)))
      (`/Game/FirstPerson/Blueprints/BP_FirstPersonGameMode.JugeChoice` _asbp_first_person_game_mode_2 true) ; ゲームモードに前進を選択した回答を渡す
    )))

(event `self.WarpFlag.OnComponentBeginOverlap`
  (params (OverlappedComponent :type "PrimitiveComponent Object Reference") (OtherActor :type "Actor Object Reference") (OtherComp :type "PrimitiveComponent Object Reference") (OtherBodyIndex :type Integer) (bFromSweep :type Boolean) (SweepResult :type "HitResult Structure (by ref)"))
  ;[1 1 1] ワープフラグ管理
  (set `self.isWarping` false) ; ワープ済みフラグを下す
)

(fn `UserConstructionScript`)