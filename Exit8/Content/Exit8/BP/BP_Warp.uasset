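; Warp actor that loops the player through the level seamlessly, keeping their relative offset when they enter the Front or Back trigger.
; Front shifts the overlapping actor to the same offset from Back, while Back mirrors it around itself in XY with a 180-degree yaw turn of actor and controller.
; Back also saves and reapplies inverted player velocity because turning zeroes it.
; An IsWarping flag blocks re-triggering until WarpFlag is overlapped.
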(event `self.Back.OnComponentBeginOverlap`
  (params (OverlappedComponent :type "PrimitiveComponent Object Reference") (OtherActor :type "Actor Object Reference") (OtherComp :type "PrimitiveComponent Object Reference") (OtherBodyIndex :type Integer) (bFromSweep :type Boolean) (SweepResult :type "HitResult Structure (by ref)"))
  (bind (_returnvalue_roll _returnvalue_pitch _returnvalue_yaw) (`KismetMathLibrary.BreakRotator` (`self.K2_GetActorRotation` OtherActor)))
  (bind _returnvalue (`GameplayStatics.GetPlayerController` 0))
  (bind (_returnvalue_roll_2 _returnvalue_pitch_2 _returnvalue_yaw_2) (`KismetMathLibrary.BreakRotator` (`Controller.GetControlRotation` _returnvalue)))
  (if (not (`self.isWarping`))
    (set `self.isWarping` true)
    (set `self.Velocity` (`MovementComponent.Velocity` (`Pawn.GetMovementComponent` (`GameplayStatics.GetPlayerPawn` 0))))
    (`self.K2_SetActorLocationAndRotation` OtherActor (+ (* (- (`self.K2_GetActorLocation` OtherActor) (`SceneComponent.K2_GetComponentLocation` (`self.Back`))) (-1.0 -1.0 1.0)) (`SceneComponent.K2_GetComponentLocation` (`self.Back`))) (`KismetMathLibrary.MakeRotator` _returnvalue_roll _returnvalue_pitch (+ _returnvalue_yaw 180.0)) false true)
    (`Controller.SetControlRotation` _returnvalue (`KismetMathLibrary.MakeRotator` _returnvalue_roll_2 _returnvalue_pitch_2 (+ _returnvalue_yaw_2 180.0)))
    (set `MovementComponent.Velocity` (* (`self.Velocity`) (-1.0 -1.0 1.0)) (`Pawn.GetMovementComponent` (`GameplayStatics.GetPlayerPawn` 0))) ; 反転すると速度が0になるので対策
  ))

(event `self.Front.OnComponentBeginOverlap`
  (params (OverlappedComponent :type "PrimitiveComponent Object Reference") (OtherActor :type "Actor Object Reference") (OtherComp :type "PrimitiveComponent Object Reference") (OtherBodyIndex :type Integer) (bFromSweep :type Boolean) (SweepResult :type "HitResult Structure (by ref)"))
  (if (not (`self.isWarping`))
    (set `self.isWarping` true)
    (`self.K2_SetActorLocation` OtherActor (+ (- (`self.K2_GetActorLocation` OtherActor) (`SceneComponent.K2_GetComponentLocation` (`self.Front`))) (`SceneComponent.K2_GetComponentLocation` (`self.Back`))) false false)))

(event `self.WarpFlag.OnComponentBeginOverlap`
  (params (OverlappedComponent :type "PrimitiveComponent Object Reference") (OtherActor :type "Actor Object Reference") (OtherComp :type "PrimitiveComponent Object Reference") (OtherBodyIndex :type Integer) (bFromSweep :type Boolean) (SweepResult :type "HitResult Structure (by ref)"))
  (set `self.isWarping` false))

(fn `UserConstructionScript`)